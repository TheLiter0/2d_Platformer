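; Player character for a side-scrolling platformer with flipbook animation, wall sliding, wall jumping, delayed projectile attack and score widget.
; Tick picks the flipbook from movement state and runs forward line traces while falling, slowing velocity on walls and setting left/right wall flags.
; Jump, gated by a coyote-time flag, feeds Wall Bounce, which flips yaw and launches off flagged walls.
; Enhanced Input also drives X-axis movement, a test-like launch and two hard-coded teleports.
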(event Input|EnhancedActionEvents|EnhancedInputActionIA_Jump
  (params (ActionValue :type Boolean) (ElapsedSeconds :type Float%20%28double-precision%29) (TriggeredSeconds :type Float%20%28double-precision%29) (InputAction :type Input%20Action%20Object%20Reference :default "/Game/imput/Actions/IA_Jump.IA_Jump"))
  (:Started
    (if (Variables|Default|GetIsInCoyoteTime)
      (Character|Jump)
      (|WallBounce)))
  (:Completed
    (Character|StopJumping)))

(event Input|EnhancedActionEvents|EnhancedInputActionRotate
  (params (ActionValue :type Boolean) (ElapsedSeconds :type Float%20%28double-precision%29) (TriggeredSeconds :type Float%20%28double-precision%29) (InputAction :type Input%20Action%20Object%20Reference :default "/Game/imput/Actions/Rotate.Rotate"))
  (Character|LaunchCharacter (+ (* (Transformation|GetActorForwardVector) (Variables|Default|GetWalljumpforce)) "500.000000,0.000000,1000.000000") true true))

(event Input|EnhancedActionEvents|EnhancedInputActionIA_Movement
  (params (ActionValue :type Float%20%28double-precision%29) (ElapsedSeconds :type Float%20%28double-precision%29) (TriggeredSeconds :type Float%20%28double-precision%29) (InputAction :type Input%20Action%20Object%20Reference :default "/Game/imput/Actions/IA_Movement.IA_Movement"))
  (Pawn|Input|AddMovementInput "1.000000,0.000000,0.000000" ActionValue false)
  (Pawn|SetControlRotation (Pawn|GetController) (select (> ActionValue 0.0) (Math|Rotator|MakeRotator 0.0 0.0 0.0) (Math|Rotator|MakeRotator 0.0 0.0 1.8e+02))))

(event Input|EnhancedActionEvents|EnhancedInputActionTelaport
  (params (ActionValue :type Boolean) (ElapsedSeconds :type Float%20%28double-precision%29) (TriggeredSeconds :type Float%20%28double-precision%29) (InputAction :type Input%20Action%20Object%20Reference :default "/Game/imput/Actions/Telaport.Telaport"))
  (Transformation|Teleport "4562.017851,-92.132479,-4608.963131" "0, 0, 0"))

(event Input|EnhancedActionEvents|EnhancedInputActionTelaport2
  (params (ActionValue :type Boolean) (ElapsedSeconds :type Float%20%28double-precision%29) (TriggeredSeconds :type Float%20%28double-precision%29) (InputAction :type Input%20Action%20Object%20Reference :default "/Game/imput/Actions/Telaport2.Telaport2"))
  (Transformation|Teleport "4398.063734,-81.435792,-3257.005739" "0, 0, 0"))

(event Input|EnhancedActionEvents|EnhancedInputActionAttack
  (params (ActionValue :type Boolean) (ElapsedSeconds :type Float%20%28double-precision%29) (TriggeredSeconds :type Float%20%28double-precision%29) (InputAction :type Input%20Action%20Object%20Reference :default "/Game/imput/Actions/Attack.Attack"))
  (Utilities|FlowControl|Delay 0.5)
  (Game|SpawnActorfromClass "/Game/NewFolder1/Quick_Draw_Assets/Tanuki/BP_Progectile.BP_Progectile_C" (Transformation|GetWorldTransform (Variables|Default|Getprogectilespawn)) "Undefined" "MultiplyWithRoot" 0 0))

(event EventBeginPlay
  (bind _returnvalue (UserInterface|CreateWidget "/Game/Score_system/ScoreCounter.ScoreCounter_C"))
  (UserInterface|Viewport|AddtoViewport _returnvalue 0)
  (bind _asplayer_controller (Utilities|Casting|CastToPlayerController (Pawn|GetController)))
  (Input|AddMappingContext (PlayerController|LocalPlayerSubsystems|GetEnhancedInputLocalPlayerSubsystem _asplayer_controller) "/Game/imput/IMC_Platforing.IMC_Platforing" 0 "(bIgnoreAllPressedKeysUntilRelease=True,bForceImmediately=False,bNotifyUserSettings=False)"))

(event EventTick
  (params (DeltaSeconds :type Float%20%28single-precision%29))
  (CallFunction|UpdateAnimation)
  (CallFunction|LeftWallSlide)
  (CallFunction|RightWallSlide)
  (CallFunction|RightWallSlideCheck)
  (CallFunction|LeftWallSlideCheck))

(fn ConstructionScript)

(fn UpdateAnimation
  (if (AI|Components|NavMovement|IsMovingonGround (Variables|Character|GetCharacterMovement))
    (if (> (Math|Vector|VectorLength (Transformation|GetVelocity)) 0.0)
      (Sprite|SetFlipbook (Variables|Default|GetSprite) "/Game/Paper_assets/ch/Flipbook/fb_player_run.fb_player_run")
      (else
        (Sprite|SetFlipbook (Variables|Default|GetSprite) "/Game/Paper_assets/ch/Flipbook/fb_play_IDLE.fb_play_IDLE")))
    (elif (< (.z (Transformation|GetVelocity)) -1e+02)
      (Sprite|SetFlipbook (Variables|Default|GetSprite) "/Game/Paper_assets/ch/Flipbook/fb_player_fall.fb_player_fall")
      (else
        (Sprite|SetFlipbook (Variables|Default|GetSprite) "/Game/Paper_assets/ch/Flipbook/fb_player_jumprise.fb_player_jumprise")))))

(fn WallJump
  (if (Variables|Default|GetbIsTouchingWall)
    (Variables|Default|SetJumpMaxCount (+ (Variables|Default|GetJump%20Max%20Count) 3))
    (else
      (Variables|Default|SetJumpMaxCount (Variables|Default|GetJump%20Max%20Count)))))

(fn LeftWallSlide
  (bind _capsulecomponent (Variables|Collision|GetCapsuleComponent))
  (bind _charactermovement (Variables|Character|GetCharacterMovement))
  (bind _returnvalue (Transformation|GetWorldLocation _capsulecomponent))
  (if (AI|Components|NavMovement|IsFalling (Variables|Character|GetCharacterMovement))
    (bind _output_get (Variables|Default|SetNewVar_1 _returnvalue))
    (bind _returnvalue_2 (Collision|LineTraceByChannel (Math|Vector|MakeVector (.x _output_get) (.y _output_get) (.z _output_get)) (- (+ _returnvalue (* (Math|Vector|GetForwardVector _capsulecomponent) (Variables|Character|GetWall%20check%20Distense))) "10.000000,0.000000,0.000000") "TraceTypeQuery3" true 0 "None" true "(R=1.000000,G=0.000000,B=0.000000,A=1.000000)" "(R=0.000000,G=1.000000,B=0.000000,A=1.000000)" 0.5))
    (if _returnvalue_2
      (Variables|Default|SetleftWallJump? true)
      (Variables|/Script/Engine.MovementComponent|SetVelocity _charactermovement (Math|Interpolation|VInterptoConstant (Variables|/Script/Engine.MovementComponent|GetVelocity _charactermovement) "0, 0, 0" (Utilities|Time|GetWorldDeltaSeconds) 2.2e+03))
      (else
        (Variables|Default|SetleftWallJump? false)))))

(fn WallSlide2
  (bind _capsulecomponent (Variables|Collision|GetCapsuleComponent))
  (bind _charactermovement (Variables|Character|GetCharacterMovement))
  (bind _returnvalue (Transformation|GetWorldLocation _capsulecomponent))
  (if (AI|Components|NavMovement|IsFalling (Variables|Character|GetCharacterMovement))
    (bind _returnvalue_2 (Collision|LineTraceByChannel _returnvalue (+ _returnvalue (* (Math|Vector|GetForwardVector _capsulecomponent) (Variables|Character|GetWall%20check%20Distense))) "TraceTypeQuery3" true 0 "Persistent" false))
    (if _returnvalue_2
      (Variables|Default|SetRightWallJump? true)
      (Variables|/Script/Engine.MovementComponent|SetVelocity _charactermovement (Math|Interpolation|VInterptoConstant (Variables|/Script/Engine.MovementComponent|GetVelocity _charactermovement) "0, 0, 0" (Utilities|Time|GetWorldDeltaSeconds) 2.2e+03))
      (else
        (Variables|Default|SetRightWallJump? false :!label _label)))
    (else
      (goto _label))))

(fn RightWallSlide
  (bind _capsulecomponent (Variables|Collision|GetCapsuleComponent))
  (bind _charactermovement (Variables|Character|GetCharacterMovement))
  (bind _returnvalue (Transformation|GetWorldLocation _capsulecomponent))
  (if (AI|Components|NavMovement|IsFalling (Variables|Character|GetCharacterMovement))
    (bind _output_get (Variables|Default|SetNewVar_0 _returnvalue))
    (bind _returnvalue_2 (Collision|LineTraceByChannel (Math|Vector|MakeVector (+ (.x _output_get) 2e+01) (.y _output_get) (- (.z _output_get) 0.0)) (- (+ _returnvalue (* (Math|Vector|GetForwardVector _capsulecomponent) (Variables|Character|GetWall%20check%20Distense))) "-10.000000,0.000000,0.000000") "TraceTypeQuery3" true 0 "None" false "(R=0.000000,G=0.311743,B=1.000000,A=1.000000)" "(R=0.000000,G=1.000000,B=0.000000,A=1.000000)" 0.5))
    (if _returnvalue_2
      (Variables|Default|SetRightWallJump? true)
      (Variables|/Script/Engine.MovementComponent|SetVelocity _charactermovement (Math|Interpolation|VInterptoConstant (Variables|/Script/Engine.MovementComponent|GetVelocity _charactermovement) "0, 0, 0" (Utilities|Time|GetWorldDeltaSeconds) 2.2e+03))
      (else
        (Variables|Default|SetRightWallJump? false)))))

(fn LeftWallSlideCheck
  (bind _capsulecomponent (Variables|Collision|GetCapsuleComponent))
  (bind _returnvalue (Transformation|GetWorldLocation _capsulecomponent))
  (if (AI|Components|NavMovement|IsFalling (Variables|Character|GetCharacterMovement))
    (bind _output_get (Variables|Default|SetNewVar_1 _returnvalue))
    (bind _returnvalue_2 (Collision|LineTraceByChannel (Math|Vector|MakeVector (.x _output_get) (.y _output_get) (.z _output_get)) (- (+ _returnvalue (* (Math|Vector|GetForwardVector _capsulecomponent) (Variables|Character|GetWall%20check%20Distense))) "10.000000,0.000000,0.000000") "TraceTypeQuery3" true 0 "None" true "(R=1.000000,G=0.000000,B=0.000000,A=1.000000)" "(R=0.000000,G=1.000000,B=0.000000,A=1.000000)" 0.5))
    (if _returnvalue_2
      (Variables|Default|SetWallCheckLeft true)
      (else
        (Variables|Default|SetWallCheckLeft false)))))

(fn RightWallSlideCheck
  (bind _capsulecomponent (Variables|Collision|GetCapsuleComponent))
  (bind _returnvalue (Transformation|GetWorldLocation _capsulecomponent))
  (if (AI|Components|NavMovement|IsFalling (Variables|Character|GetCharacterMovement))
    (bind _output_get (Variables|Default|SetNewVar_0 _returnvalue))
    (bind _returnvalue_2 (Collision|LineTraceByChannel (Math|Vector|MakeVector (+ (.x _output_get) 2e+01) (.y _output_get) (- (.z _output_get) 1e+01)) (- (+ _returnvalue (* (Math|Vector|GetForwardVector _capsulecomponent) (Variables|Character|GetWall%20check%20Distense))) "-10.000000,0.000000,0.000000") "TraceTypeQuery3" true 0 "None" false "(R=0.000000,G=0.311743,B=1.000000,A=1.000000)" "(R=0.000000,G=1.000000,B=0.000000,A=1.000000)" 0.5))
    (if _returnvalue_2
      (Variables|Default|SetWallCheckRight false)
      (else
        (Variables|Default|SetWallCheckRight true)))))

(fn TouchingGround
  (bind _capsulecomponent (Variables|Collision|GetCapsuleComponent))
  (bind _returnvalue (Transformation|GetWorldLocation _capsulecomponent))
  (bind _output_get (Variables|Default|SetNewVar_0 _returnvalue))
  (bind _returnvalue_2 (Collision|LineTraceByChannel (Math|Vector|MakeVector (.x _output_get) (.y _output_get) (- (.z _output_get) 9e+01)) (- (+ _returnvalue (* (Math|Vector|GetForwardVector _capsulecomponent) (Variables|Character|GetWall%20check%20Distense))) "0.000000,0.000000,90.000000") "TraceTypeQuery3" true 0 "None" false "(R=1.000000,G=0.946137,B=0.303640,A=1.000000)" "(R=0.000000,G=1.000000,B=0.000000,A=1.000000)" 0.5))
  (Variables|Default|SetTouchingGround? _returnvalue_2))

(event OnComponentBeginOverlap(Capsule1)
  (params (OverlappedComponent :type Primitive%20Component%20Object%20Reference) (OtherActor :type Actor%20Object%20Reference) (OtherComp :type Primitive%20Component%20Object%20Reference) (OtherBodyIndex :type Integer) (bFromSweep :type Boolean) (SweepResult :type Hit%20Result%20Structure%20%28by%20ref%29))
  (Variables|Default|SetbIsTouchingWall true))

(event OnComponentBeginOverlap(Capsule)
  (params (OverlappedComponent :type Primitive%20Component%20Object%20Reference) (OtherActor :type Actor%20Object%20Reference) (OtherComp :type Primitive%20Component%20Object%20Reference) (OtherBodyIndex :type Integer) (bFromSweep :type Boolean) (SweepResult :type Hit%20Result%20Structure%20%28by%20ref%29))
  (Variables|Default|SetbIsTouchingWall true))

(event OnComponentEndOverlap(Capsule)
  (params (OverlappedComponent :type Primitive%20Component%20Object%20Reference) (OtherActor :type Actor%20Object%20Reference) (OtherComp :type Primitive%20Component%20Object%20Reference) (OtherBodyIndex :type Integer))
  (Variables|Default|SetbIsTouchingWall false))

(event OnComponentEndOverlap(Capsule1)
  (params (OverlappedComponent :type Primitive%20Component%20Object%20Reference) (OtherActor :type Actor%20Object%20Reference) (OtherComp :type Primitive%20Component%20Object%20Reference) (OtherBodyIndex :type Integer))
  (Variables|Default|SetbIsTouchingWall false))